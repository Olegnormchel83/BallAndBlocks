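; BP_BlockDistructibleScalableColorable is a child Blueprint of a block obstacle that changes color when hit by the ball.
; On actor overlap it runs the parent logic, then checks whether the other actor is a BP_Ball.
; The first ball overlap swaps the Cube's material to BasicAsset01 and sets the ColorChanged flag, so the swap happens only once.
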(event EventBeginPlay
  (|CallParentFunction) ; This node is disabled and will not be called.\nDrag off pins to build functionality.
)

(event Collision|EventActorBeginOverlap
  (params (OtherActor :type Actor%20Object%20Reference))
  (|CallParentFunction OtherActor)
  (Utilities|Casting|CastToBP_Ball OtherActor)
  (if (not (Variables|Default|GetColorChanged))
    (Rendering|Material|SetMaterial (Variables|Default|GetCube) 0 "/Engine/MapTemplates/Materials/BasicAsset01.BasicAsset01")
    (Variables|Default|SetColorChanged true)))

(event EventTick
  (params (DeltaSeconds :type Float%20%28single-precision%29))
  (|CallParentFunction DeltaSeconds) ; This node is disabled and will not be called.\nDrag off pins to build functionality.
)

(fn ConstructionScript
  (|CallParentFunction))