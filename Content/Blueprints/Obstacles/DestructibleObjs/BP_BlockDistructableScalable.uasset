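; A destructible block obstacle that shrinks each time a BP_Ball overlaps it.
; BeginPlay stores the starting scale, and each ball overlap subtracts that scale times ScaleRatio, so the block shrinks in equal linear steps.
; Begin play and overlap first call the parent implementation; this graph sets no minimum scale and does not destroy the block itself.
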(event EventBeginPlay
  (|CallParentFunction)
  (Variables|Default|SetMainScale (Transformation|GetActorScale3D)))

(event Collision|EventActorBeginOverlap
  (params (OtherActor :type Actor%20Object%20Reference))
  (|CallParentFunction OtherActor)
  (Utilities|Casting|CastToBP_Ball OtherActor)
  (Transformation|SetActorScale3D (- (Transformation|GetActorScale3D) (* (Variables|Default|GetMainScale) (Variables|Default|GetScaleRatio)))))

(event EventTick
  (params (DeltaSeconds :type Float%20%28single-precision%29))
  (|CallParentFunction DeltaSeconds) ; This node is disabled and will not be called.\nDrag off pins to build functionality.
)

(fn ConstructionScript
  (|CallParentFunction))